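; AI controller for Zombie_BP that runs a Tick-driven state machine: Idle, Patrol, Meet, Trace, Attack and Death.
; Idle and Patrol use timers and random rolls to wander to nearby points, switching to Meet when the pawn's TracePlayer flag is set.
; Trace chases the target until it is within attack range or lost, while pawn flags end Meet and Attack.
; ChangeState forwards each state to the pawn, and zero HP forces Death.
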(event `self.ReceiveBeginPlay`
  (bind _aszombie_bp (cast `/Game/SM_Project/BluePrint/Zombie_BP` (`self.K2_GetPawn`)))
  (set `self.ZombieActor` _aszombie_bp))

(event `self.ReceiveTick`
  (params (DeltaSeconds :type "Float (single-precision)"))
  (if (<= (`/Game/SM_Project/BluePrint/Zombie_BP.HP` (`self.ZombieActor`)) 0.0)
    (`self.ChangeState` "NewEnumerator3")
    (else
      (switch `/Game/SM_Project/BluePrint/EZombieState` (`self.CurrentState`)
        (:`NewEnumerator0`
          (`self.State_Idle`))
        (:`NewEnumerator1`
          (`self.State_Trace`))
        (:`NewEnumerator2`
          (`self.State_Attack`))
        (:`NewEnumerator3`
          (`self.State_Death`))
        (:`NewEnumerator4`
          (`self.State_Patrol`))
        (:`NewEnumerator5`
          (`self.State_Meet`))))))

(fn `ChangeState`
  (params (NewState :type "/Game/SM_Project/BluePrint/EZombieState Enum"))
  (bind _output_get (set `self.CurrentState` NewState))
  (bind _aszombie_bp (cast `/Game/SM_Project/BluePrint/Zombie_BP` (`self.K2_GetPawn`)))
  (`/Game/SM_Project/BluePrint/Zombie_BP.NewState` _aszombie_bp _output_get))

(fn `GetState`
  (returns (CurrentState :type "/Game/SM_Project/BluePrint/EZombieState Enum"))
  (return (`self.CurrentState`)))

(fn `State_Attack`
  (bind _zombieactor (`self.ZombieActor`))
  (`self.StopMovement`)
  (if (`/Game/SM_Project/BluePrint/Zombie_BP.EndAttackMotion` _zombieactor)
    (set `/Game/SM_Project/BluePrint/Zombie_BP.EndAttackMotion` false _zombieactor)
    (`self.ChangeState` "NewEnumerator1")))

(fn `State_Death`)

(fn `State_Idle`
  (if (`/Game/SM_Project/BluePrint/Zombie_BP.TracePlayer` (`self.ZombieActor`))
    (`self.ChangeState` "NewEnumerator5")
    (else
      (bind _output_get (set `self.CurrentChangeTime` (+ (`self.CurrentChangeTime`) (`GameplayStatics.GetWorldDeltaSeconds`))))
      (if (>= _output_get (`self.ChangePatrolTime`))
        (set `self.CurrentChangeTime` 0.0)
        (switch `int` (`KismetMathLibrary.RandomInteger` 2)
          (:`0`
            (`self.ChangeState` "NewEnumerator4")))))))

(fn `State_Meet`
  (if (`/Game/SM_Project/BluePrint/Zombie_BP.MeetingEnd` (`self.ZombieActor`))
    (set `/Game/SM_Project/BluePrint/Zombie_BP.MeetingEnd` false (`self.ZombieActor`))
    (`self.ChangeState` "NewEnumerator1")))

(fn `State_Patrol`
  (if (`/Game/SM_Project/BluePrint/Zombie_BP.TracePlayer` (`self.ZombieActor`))
    (`self.ChangeState` "NewEnumerator5")
    (else
      (bind _output_get (set `self.CurrentChangeTime` (+ (`self.CurrentChangeTime`) (`GameplayStatics.GetWorldDeltaSeconds`))))
      (if (>= _output_get (`self.PatrolTime`))
        (bind _returnvalue (`self.MoveToLocation` (`self.RandomLocation`) 10.0 true true true))
        (if (`|EnumEquality` _returnvalue "AlreadyAtGoal")
          (set `self.CurrentChangeTime` 0.0)
          (switch `int` (`KismetMathLibrary.RandomInteger` 2)
            (:`0`
              (`self.ChangeState` "NewEnumerator0")))
          (else
            (set `self.CurrentPatrolTime` (+ (`self.CurrentPatrolTime`) (`GameplayStatics.GetWorldDeltaSeconds`)))
            (if (>= (`self.CurrentPatrolTime`) (`self.PatrolTime`))
              (set `self.CurrentPatrolTime` 0.0)
              (set `self.CurrentChangeTime` 0.0))))
        (else
          (set `self.RandomLocation` (+ (`self.K2_GetActorLocation` (`self.ZombieActor`)) (`KismetMathLibrary.MakeVector` (`KismetMathLibrary.RandomFloatInRange` -1000.0 1000.0) (`KismetMathLibrary.RandomFloatInRange` -1000.0 1000.0)))))))))

(fn `State_Trace`
  (locals (L_TargetDistance :type "Float (double-precision)" :default 0.0))
  (bind _zombieactor (`self.ZombieActor`))
  (set `local.L_TargetDistance` (`KismetMathLibrary.VSize` (- (`self.K2_GetActorLocation` (`self.ZombieActor`)) (`self.K2_GetActorLocation` (`/Game/SM_Project/BluePrint/Zombie_BP.TargetActor` (`self.ZombieActor`))))))
  (if (<= (`local.L_TargetDistance`) (`self.TraceDistance`))
    (if (<= (`local.L_TargetDistance`) (`self.AttackDistance`))
      (`self.ChangeState` "NewEnumerator2")
      (else
        (`NavigationSystem.SimpleMoveToActor` self (`/Game/SM_Project/BluePrint/Zombie_BP.TargetActor` (`self.ZombieActor`)))))
    (else
      (set `/Game/SM_Project/BluePrint/Zombie_BP.TargetActor` null _zombieactor)
      (set `/Game/SM_Project/BluePrint/Zombie_BP.TracePlayer` false _zombieactor)
      (`self.ChangeState` "NewEnumerator0"))))

(fn `UserConstructionScript`)