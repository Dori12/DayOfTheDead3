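; Zombie enemy Blueprint that detects the player and deals melee damage through hand collisions.
; PawnSensing sight or hearing stores the first detected player as TargetActor and latches TracePlayer.
; Left and right hand overlaps apply AttackDamage while ZombieAttack is set, then clear it; only the left checks for the player class.
; Incoming damage lowers HP, while separate events set CurrentState and destroy the actor on death.
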(event `self.PawnSensing.OnSeePawn`
  (params (Pawn :type "Pawn Object Reference"))
  (if (not (`self.TracePlayer`))
    (bind _asblueprint_player (cast `/Game/Fix_Version/Player/Blueprint_Player` Pawn))
    (set `self.TargetActor` _asblueprint_player)
    (set `self.TracePlayer` true)))

(event `self.PawnSensing.OnHearNoise`
  (params (Instigator :type "Pawn Object Reference") (Location :type "Vector Structure (by ref)") (Volume :type "Float (single-precision)"))
  (if (not (`self.TracePlayer`))
    (bind _asblueprint_player (cast `/Game/Fix_Version/Player/Blueprint_Player` Instigator))
    (set `self.TargetActor` _asblueprint_player)
    (set `self.TracePlayer` true)))

(event `self.LeftCollision.OnComponentBeginOverlap`
  (params (OverlappedComponent :type "PrimitiveComponent Object Reference") (OtherActor :type "Actor Object Reference") (OtherComp :type "PrimitiveComponent Object Reference") (OtherBodyIndex :type Integer) (bFromSweep :type Boolean) (SweepResult :type "HitResult Structure (by ref)"))
  (if (`self.ZombieAttack`)
    (bind _asblueprint_player (cast `/Game/Fix_Version/Player/Blueprint_Player` OtherActor))
    (`GameplayStatics.ApplyDamage` _asblueprint_player (`self.AttackDamage`))
    (set `self.ZombieAttack` false)))

(event `self.RightCollision.OnComponentBeginOverlap`
  (params (OverlappedComponent :type "PrimitiveComponent Object Reference") (OtherActor :type "Actor Object Reference") (OtherComp :type "PrimitiveComponent Object Reference") (OtherBodyIndex :type Integer) (bFromSweep :type Boolean) (SweepResult :type "HitResult Structure (by ref)"))
  (if (`self.ZombieAttack`)
    (`GameplayStatics.ApplyDamage` OtherActor (`self.AttackDamage`))
    (set `self.ZombieAttack` false)))

(event `NewState`
  (params (NewState :type "/Game/SM_Project/BluePrint/EZombieState Enum"))
  (set `self.CurrentState` NewState))

(event `self.ReceiveAnyDamage`
  (params (Damage :type "Float (single-precision)") (DamageType :type "DamageType Object Reference") (InstigatedBy :type "Controller Object Reference") (DamageCauser :type "Actor Object Reference"))
  (set `self.HP` (- (`self.HP`) Damage)))

(event `Death`
  (`self.K2_DestroyActor`))

(fn `UserConstructionScript`)