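; Inventory component that stores items as objects in a fixed-size slot array, filled on BeginPlay with BP_InvItem_Empty placeholders that mark free slots.
; AddItem tops up a matching stack and moves overflow into a new object in the first empty slot, though its space check always reports true.
; Slot getters and setters support swaps within or between inventories.
; RemoveItem replaces the first depleted item with a placeholder and refreshes InventoryPanel.
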(event `self.ReceiveBeginPlay`
  (`self.InventoryInitialize`))

(fn `AddItem`
  (params (ItemClass :type "/Game/SM_Project/InventorySample/BluePrints/Inventory/Items/BP_InvItem Class Reference") (AddToAmount :type Integer))
  (returns (`Add Item?` :type Boolean))
  (locals (L_Class :type "/Game/SM_Project/InventorySample/BluePrints/Inventory/Items/BP_InvItem Class Reference") (L_Amount :type Integer) (L_OpenSpace :type Integer) (L_Item :type "/Game/SM_Project/InventorySample/BluePrints/Inventory/Items/BP_InvItem Object Reference") (L_Index :type Integer))
  (bind (_has_space_ _openspaces) (`self.HasSapceInInventory`))
  (bind _l_item (`local.L_Item`))
  (bind _l_item_2 (`local.L_Item`))
  (bind _l_item_3 (`local.L_Item`))
  (set `local.L_Class` ItemClass)
  (set `local.L_Amount` AddToAmount)
  (if _has_space_
    (set `local.L_OpenSpace` _openspaces)
    (for _array_element (`self.InventoryItem`)
      (if (== (`GameplayStatics.GetObjectClass` _array_element) (`local.L_Class`))
        (bind _output_get (set `local.L_Item` _array_element))
        (if (`/Game/SM_Project/InventorySample/BluePrints/Inventory/Items/BP_InvItem.GetCanStack?` _output_get)
          (if (> (`/Game/SM_Project/InventorySample/BluePrints/Inventory/Items/BP_InvItem.HasRoomOnStack` (`local.L_Item`)) 0)
            (if (<= (+ (`/Game/SM_Project/InventorySample/BluePrints/Inventory/Items/BP_InvItem.GetAmount` _l_item_2) (`local.L_Amount`)) (`/Game/SM_Project/InventorySample/BluePrints/Inventory/Items/BP_InvItem.GetMaxStack` _l_item_2))
              (`/Game/SM_Project/InventorySample/BluePrints/Inventory/Items/BP_InvItem.SetAmount` _l_item_3 (+ (`/Game/SM_Project/InventorySample/BluePrints/Inventory/Items/BP_InvItem.GetAmount` _l_item_3) (`local.L_Amount`)))
              (return true)
              (elif (> (`local.L_OpenSpace`) 0)
                (set `local.L_Amount` (- (`local.L_Amount`) (`/Game/SM_Project/InventorySample/BluePrints/Inventory/Items/BP_InvItem.HasRoomOnStack` (`local.L_Item`))))
                (`/Game/SM_Project/InventorySample/BluePrints/Inventory/Items/BP_InvItem.SetAmount` _l_item (`/Game/SM_Project/InventorySample/BluePrints/Inventory/Items/BP_InvItem.GetMaxStack` _l_item))
                (for (_array_element_2 _array_index) (`self.InventoryItem`) :!label _label
                  (if (== (`GameplayStatics.GetObjectClass` _array_element_2) "/Game/SM_Project/InventorySample/BluePrints/Inventory/Items/BP_InvItem_Empty.BP_InvItem_Empty_C")
                    (set `local.L_Index` _array_index)
                    (break)
                    (else
                      (set `local.L_Index` -1))))
                (if (>= (`local.L_Index`) 0)
                  (bind _returnvalue (`|GenericCreateObject` (`local.L_Class`) self))
                  (`/Game/SM_Project/InventorySample/BluePrints/Inventory/Items/BP_InvItem.SetAmount` _returnvalue (`local.L_Amount`))
                  (`KismetArrayLibrary.Array_Set` (`self.InventoryItem`) (`local.L_Index`) _returnvalue)
                  (return true)
                  (else
                    (return false)))
                (else
                  (return false)))))
          (else
            (goto _label)))))
    (goto _label)
    (else
      (return false))))

(fn `GetInventory`
  (returns (InventoryComponent :type "Array of /Game/SM_Project/InventorySample/BluePrints/Inventory/Items/BP_InvItem Object Reference"))
  (return (`self.InventoryItem`)))

(fn `GetItemInSlot`
  (params (index :type Integer))
  (returns (Item :type "/Game/SM_Project/InventorySample/BluePrints/Inventory/Items/BP_InvItem Object Reference"))
  (bind _output (`|GetArrayItem` (`self.InventoryItem`) index))
  (`/Engine/EditorBlueprintResources/StandardMacros.IsValid` _output
    (:`Is Valid`
      (return _output))
    (:`Is Not Valid`
      (return null))))

(fn `HasSapceInInventory`
  (returns (`Has Space?` :type Boolean) (OpenSpaces :type Integer))
  (locals (L_OpenSpaces :type Integer))
  (for _array_element (`self.InventoryItem`)
    (if (== (`GameplayStatics.GetObjectClass` _array_element) "/Game/SM_Project/InventorySample/BluePrints/Inventory/Items/BP_InvItem_Empty.BP_InvItem_Empty_C")
      (`/Engine/EditorBlueprintResources/StandardMacros.IncrementInt` (`local.L_OpenSpaces`))))
  (return true (`local.L_OpenSpaces`)))

(fn `InventoryInitialize`
  (`KismetArrayLibrary.Array_Clear` (`self.InventoryItem`))
  (for _ (range (`self.Sltos`))
    (bind _returnvalue (`|GenericCreateObject` "/Game/SM_Project/InventorySample/BluePrints/Inventory/Items/BP_InvItem_Empty.BP_InvItem_Empty_C" self))
    (`KismetArrayLibrary.Array_Add` (`self.InventoryItem`) _returnvalue)))

(fn `RemoveItem`
  (returns (RemoveSuccess :type Boolean))
  (for (_array_element _array_index) (`self.InventoryItem`)
    (if (!= (`GameplayStatics.GetObjectClass` _array_element) "/Game/SM_Project/InventorySample/BluePrints/Inventory/Items/BP_InvItem_Empty.BP_InvItem_Empty_C")
      (if (<= (`/Game/SM_Project/InventorySample/BluePrints/Inventory/Items/BP_InvItem.GetAmount` _array_element) 0)
        (bind _returnvalue (`|GenericCreateObject` "/Game/SM_Project/InventorySample/BluePrints/Inventory/Items/BP_InvItem_Empty.BP_InvItem_Empty_C" self))
        (`KismetArrayLibrary.Array_Set` (`self.InventoryItem`) _array_index _returnvalue)
        (`/Game/SM_Project/InventorySample/UI/Widget_InventoryPanel.Initialize` (`self.Inventory Panel`))
        (return true))))
  (return false))

(fn `SetSlotInInventory`
  (params (Item :type "/Game/SM_Project/InventorySample/BluePrints/Inventory/Items/BP_InvItem Object Reference") (Index :type Integer))
  (returns (`Success?` :type Boolean))
  (if (<= Index (`KismetArrayLibrary.Array_LastIndex` (`self.InventoryItem`)))
    (`KismetArrayLibrary.Array_Set` (`self.InventoryItem`) Index Item)
    (return true)
    (else
      (return false))))

(fn `SwapItems`
  (params (fromIndex :type Integer) (fromItem :type "/Game/SM_Project/InventorySample/BluePrints/Inventory/InventoryComponent Object Reference") (toIndex :type Integer) (toItem :type "/Game/SM_Project/InventorySample/BluePrints/Inventory/InventoryComponent Object Reference"))
  (locals (L_FromItem :type "/Game/SM_Project/InventorySample/BluePrints/Inventory/Items/BP_InvItem Object Reference") (L_ToItem :type "/Game/SM_Project/InventorySample/BluePrints/Inventory/Items/BP_InvItem Object Reference"))
  (set `local.L_FromItem` (`self.GetItemInSlot` fromItem fromIndex))
  (set `local.L_ToItem` (`self.GetItemInSlot` toItem toIndex))
  (`self.SetSlotInInventory` toItem (`local.L_FromItem`) toIndex)
  (`self.SetSlotInInventory` fromItem (`local.L_ToItem`) fromIndex))