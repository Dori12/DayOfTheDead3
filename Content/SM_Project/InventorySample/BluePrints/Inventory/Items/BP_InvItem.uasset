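; BP_InvItem is an inventory item that restores either the player's HP or Energy.
; Getters read stacking rules, item info and world actor from the DB_InventoryItem data table by RowName.
; OnUse starts use on Blueprint_Player if the relevant stat is below maximum, then Consume decrements the amount, updates the inventory and applies HealAmount.
; Energy caps at a hardcoded limit, while the HP clamp never runs; OnDrop is empty.
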(fn `Consume`
  (params (UsePlayer :type "PlayerController Object Reference"))
  (locals (L_PlayerCharacter :type "/Game/Fix_Version/Player/Blueprint_Player Object Reference"))
  (bind _l_playercharacter (`local.L_PlayerCharacter`))
  (bind _l_playercharacter_2 (`local.L_PlayerCharacter`))
  (bind _l_playercharacter_3 (`local.L_PlayerCharacter`))
  (`self.Decrease`)
  (bind _asblueprint_player (cast `/Game/Fix_Version/Player/Blueprint_Player` (`Controller.K2_GetPawn` UsePlayer)))
  (bind _output_get (set `local.L_PlayerCharacter` _asblueprint_player))
  (set `/Game/Fix_Version/Player/Blueprint_Player.UsingItem` null _output_get)
  (set `/Game/Fix_Version/Player/Blueprint_Player.UseItem?` false _output_get)
  (if (`self.IsHeal?`)
    (bind _output_get_2 (set `/Game/Fix_Version/Player/Blueprint_Player.CurrentHP` (+ (`/Game/Fix_Version/Player/Blueprint_Player.CurrentHP` _l_playercharacter) (`self.HealAmount`)) _l_playercharacter))
    (if false
      (set `/Game/Fix_Version/Player/Blueprint_Player.CurrentHP` (`/Game/Fix_Version/Player/Blueprint_Player.MaxHP` _l_playercharacter_3) _l_playercharacter_3))
    (else
      (bind _output_get_3 (set `/Game/Fix_Version/Player/Blueprint_Player.Energy` (+ (`/Game/Fix_Version/Player/Blueprint_Player.Energy` _l_playercharacter_2) (`self.HealAmount`)) _l_playercharacter_2))
      (if (>= _output_get_3 150.0)
        (set `/Game/Fix_Version/Player/Blueprint_Player.Energy` 150.0 (`local.L_PlayerCharacter`))))))

(fn `Decrease`
  (`/Engine/EditorBlueprintResources/StandardMacros.DecrementInt` (`self.Amount`)
    (:`  `
      (`/Game/SM_Project/InventorySample/UI/Widget_InventorySlot.SetStyle` (`self.UseWidget`))
      (`/Game/SM_Project/InventorySample/BluePrints/Inventory/InventoryComponent.RemoveItem` (`/Game/SM_Project/InventorySample/UI/Widget_InventorySlot.InventoryComponent` (`self.UseWidget`))))))

(fn `GetAmount`
  (returns (Amount :type Integer))
  (return (`self.Amount`)))

(fn `GetCanStack?`
  (returns (`Can Stack?` :type Boolean))
  (bind _returnvalue (`|GetDataTableRow` "/Game/SM_Project/InventorySample/Enumerator/DB_InventoryItem.DB_InventoryItem" (`self.RowName`))
    (:`then`
      (return (`.CanStack?_13_982950D14BD422CD99C6C58800BB8707` (break `/Game/SM_Project/InventorySample/BluePrints/Inventory/SInventoryItemInfo` _returnvalue))))
    (:`RowNotFound`
      (return false))))

(fn `GetInventoryItemInfo`
  (returns (InventoryItemInfo :type "/Game/SM_Project/InventorySample/BluePrints/Inventory/SInventoryItemInfo Structure"))
  (bind _returnvalue (`|GetDataTableRow` "/Game/SM_Project/InventorySample/Enumerator/DB_InventoryItem.DB_InventoryItem" (`self.RowName`))
    (:`then`
      (return _returnvalue))
    (:`RowNotFound`
      (return))))

(fn `GetItemInfo`
  (returns (`Item Info` :type "/Game/SM_Project/InventorySample/BluePrints/Inventory/SItemInfo Structure"))
  (bind _returnvalue (`|GetDataTableRow` "/Game/SM_Project/InventorySample/Enumerator/DB_InventoryItem.DB_InventoryItem" (`self.RowName`))
    (:`then`
      (return (break `/Game/SM_Project/InventorySample/BluePrints/Inventory/SInventoryItemInfo` _returnvalue)))
    (:`RowNotFound`
      (return))))

(fn `GetMaxStack`
  (returns (MaxStack :type Integer))
  (bind _returnvalue (`|GetDataTableRow` "/Game/SM_Project/InventorySample/Enumerator/DB_InventoryItem.DB_InventoryItem" (`self.RowName`))
    (:`then`
      (return (`.MaxStack_17_1ABE1B604FF023CA621A759052587E77` (break `/Game/SM_Project/InventorySample/BluePrints/Inventory/SInventoryItemInfo` _returnvalue))))
    (:`RowNotFound`
      (return 0))))

(fn `GetWorldActor`
  (returns (WorldActor :type "Actor Class Reference"))
  (bind _returnvalue (`|GetDataTableRow` "/Game/SM_Project/InventorySample/Enumerator/DB_InventoryItem.DB_InventoryItem" (`self.RowName`))
    (:`then`
      (return (`.WorldActor_19_E0F892704BF5F5A755D9EB93BA13B06F` (break `/Game/SM_Project/InventorySample/BluePrints/Inventory/SInventoryItemInfo` _returnvalue))))
    (:`RowNotFound`
      (return null))))

(fn `HasRoomOnStack`
  (returns (RoomOnStack :type Integer))
  (bind _returnvalue (`|GetDataTableRow` "/Game/SM_Project/InventorySample/Enumerator/DB_InventoryItem.DB_InventoryItem" (`self.RowName`))
    (:`then`
      (return (- (`.MaxStack_17_1ABE1B604FF023CA621A759052587E77` (break `/Game/SM_Project/InventorySample/BluePrints/Inventory/SInventoryItemInfo` _returnvalue)) (`self.Amount`))))
    (:`RowNotFound`
      (return -1))))

(fn `OnDrop`)

(fn `OnUse`
  (params (UsePlayer :type "PlayerController Object Reference") (UseWidget :type "/Game/SM_Project/InventorySample/UI/Widget_InventorySlot Object Reference"))
  (locals (L_PlayerCharacter :type "/Game/Fix_Version/Player/Blueprint_Player Object Reference"))
  (bind _l_playercharacter (`local.L_PlayerCharacter`))
  (if (== (`self.UseWidget`) null)
    (set `self.UseWidget` UseWidget))
  (bind _asblueprint_player (cast `/Game/Fix_Version/Player/Blueprint_Player` (`Controller.K2_GetPawn` UsePlayer))
    (:`then`
      (bind _output_get (set `local.L_PlayerCharacter` _asblueprint_player))
      (if (`/Game/Fix_Version/Player/Blueprint_Player.UseItem?` _output_get)
        _
        (elif (`self.IsHeal?`)
          (if (< (`/Game/Fix_Version/Player/Blueprint_Player.CurrentHP` _l_playercharacter) (`/Game/Fix_Version/Player/Blueprint_Player.MaxHP` _l_playercharacter))
            (`/Game/Fix_Version/Player/Blueprint_Player.UseItem` (`local.L_PlayerCharacter`) self :!label _label))
          (elif (< (`/Game/Fix_Version/Player/Blueprint_Player.Energy` (`local.L_PlayerCharacter`)) 150.0)
            (goto _label)))))
    (:`CastFailed`
      (`KismetSystemLibrary.PrintString` null "BP_InvItem CLASS _ Cast [Blueprint_Player] _ FALED Function is ON Use"))))

(fn `SetAmount`
  (params (Amount :type Integer))
  (set `self.Amount` Amount))