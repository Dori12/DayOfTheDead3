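; Footprint decal actor that shows a footprint, fades it out after a delay and destroys itself.
; On BeginPlay, after a tiny delay, it applies the decal material and sort order, then creates a dynamic material instance.
; It sets the initial value on "FootOpacity", while after TimeDelay a timeline drives a differently named parameter, "FootprintOpacity", and destroys the actor on finish.
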(event `self.ReceiveBeginPlay`
  (bind _decal (`self.Decal`))
  (`KismetSystemLibrary.Delay` 0.01)
  (`DecalComponent.SetDecalMaterial` _decal (`self.FootprintDecalMaterial`))
  (`DecalComponent.SetSortOrder` _decal (`self.FootprintSortOrder`))
  (bind _returnvalue (`DecalComponent.CreateDynamicMaterialInstance` _decal))
  (`MaterialInstanceDynamic.SetScalarParameterValue` _returnvalue "FootOpacity" (`self.FootprintOriginalOpacity`))
  (`KismetSystemLibrary.Delay` (`self.TimeDelay`))
  (bind (_direction _newtrack_0) (`Timeline|Timeline_0` :!via `PlayFromStart`)
    (:`Update`
      (`MaterialInstanceDynamic.SetScalarParameterValue` _returnvalue "FootprintOpacity" _newtrack_0))
    (:`Finished`
      (`self.K2_DestroyActor`))))

(fn `UserConstructionScript`)