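; Player character component that drives surface-dependent footprints, with helpers for decals, sounds and particles.
; Footfalls trace the ground, match its physical material to an instantiated footprint type and delegate effects to it.
; Foot socket positions feed material parameter collections for tessellated imprints, written to rotating vector slots, and elastic deformation.
; Tracking carries prints and a character texture overlay onto later steps, fading by step count.
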(event `self.ReceiveBeginPlay`
  (`|ExecutionSequence`
    (:`then_0`
      ;[0.1769 0.7436 0.995 0.2] Initial Setup
      (for _array_element (`self.FootprintTypeClasses`)
        (bind _returnvalue (`|GenericCreateObject` _array_element self))
        (`KismetArrayLibrary.Array_Add` (`self.FootprintTypes`) _returnvalue)
        (bind _asblueprint_player (cast `/Game/Fix_Version/Player/Blueprint_Player` (`self.GetOwner`)))
        (set `self.CharacterReference` _asblueprint_player)))))

(event `OnFootFallEvent`
  (bind (_leftfootlocation _rightfootlocation) (`self.GetFootLocation`))
  (bind _spheremaskarrayindex (`self.SphereMaskArrayIndex`))
  (bind _mesh (`Character.Mesh` (`self.CharacterReference`)))
  (bind _z (.z (`KismetMathLibrary.MakeVector` (.x (`SceneComponent.K2_GetComponentLocation` (`Character.Mesh` (`self.CharacterReference`)))) (.y (`SceneComponent.K2_GetComponentLocation` (`Character.Mesh` (`self.CharacterReference`)))) (+ (.z (`SceneComponent.K2_GetComponentLocation` (`Character.Mesh` (`self.CharacterReference`)))) (`/Game/SM_Project/AFB/Blueprints/FootprintTypeBase.3d Kill Height` (`self.ActiveFootprintType`))))))
  ;[0.1769 0.7436 0.995 0.2] Triggered on Footfall from Anim BP
  ;[0.1769 0.7436 0.995 0.2] 3d Footprint Speed Test, Enable Tick for .4 seconds after each footstep
  (if (`/Game/SM_Project/AFB/Blueprints/FootprintTypeBase.Enable3dFootprints` (`self.ActiveFootprintType`))
    (set `self.SkipSpeedTest` false)
    (`|ExecutionSequence`
      (:`then_0`
        (`KismetSystemLibrary.Delay` 0.2)
        (set `self.SkipSpeedTest` true))
      (:`then_1`
        ;[0.1769 0.7436 0.995 0.2] Checks if Active Footprint is Valid
        (`/Engine/EditorBlueprintResources/StandardMacros.IsValid` (`self.ActiveFootprintType`)
          (:`Is Valid`
            ;[0.1769 0.7436 0.995 0.2] Checks if 3d Footpritns Are Enabled
            (if (`/Game/SM_Project/AFB/Blueprints/FootprintTypeBase.Enable3dFootprints` (`self.ActiveFootprintType`)) :!label _label
              (`|ExecutionSequence`
                (:`then_0`
                  ;[0.1769 0.7436 0.995 0.2] Allows flow through for .4 seconds after each step
                  (if (`self.SkipSpeedTest`)
                    ;[0.1769 0.7436 0.995 0.2] Speed Test
                    (if (not (>= (`KismetMathLibrary.VSize` (`CharacterMovementComponent.GetCurrentAcceleration` (`Character.CharacterMovement` (`self.CharacterReference`)))) 30.0))
                      ;[0.1769 0.7436 0.995 0.2] Stops 3d footprints spawning above set height to increase performance
                      (`/Engine/EditorBlueprintResources/StandardMacros.FlipFlop` :!label _label_2
                        (:`A`
                          (if (< (.z _leftfootlocation) _z)
                            ;[0.1769 0.7436 0.995 0.2] Gets Ball and Toe Locations
                            (for _ (range 2) :!label _label_3
                              (`/Engine/EditorBlueprintResources/StandardMacros.FlipFlop`
                                (:`A`
                                  (set `self.CurrentFootPrintLoc` (`SceneComponent.GetSocketLocation` _mesh "ball_l")))
                                (:`B`
                                  (set `self.CurrentFootPrintLoc` (`SceneComponent.GetSocketLocation` _mesh "foot_l"))))
                              ;[0.1769 0.7436 0.995 0.2] Tesselated Footprints
                              (if (== (`self.SphereMaskArrayIndex`) (`self.TessellationLoop`)) :!label _label_4
                                (set `self.SphereMaskArrayIndex` -1))
                              (set `self.SphereMaskArrayIndex` (+ _spheremaskarrayindex 1))
                              (`KismetMaterialLibrary.SetVectorParameterValue` "/Game/SM_Project/AFB/CollectionParams/ImprintFootLocations.ImprintFootLocations" (`KismetStringLibrary.Conv_StringToName` (`KismetStringLibrary.Concat_StrStr` "Vector" (`KismetStringLibrary.Conv_IntToString` (`KismetMathLibrary.Clamp` _spheremaskarrayindex 0 (`self.TessellationLoop`))))) (`KismetMathLibrary.Conv_VectorToLinearColor` (`self.CurrentFootPrintLoc`)))
                              (`KismetMaterialLibrary.SetScalarParameterValue` "/Game/SM_Project/AFB/CollectionParams/ImprintFootLocations.ImprintFootLocations" "ImprintRadius" (`/Game/SM_Project/AFB/Blueprints/FootprintTypeBase.3dRadius` (`self.ActiveFootprintType`)))
                              (`KismetMaterialLibrary.SetScalarParameterValue` "/Game/SM_Project/AFB/CollectionParams/ImprintFootLocations.ImprintFootLocations" "ImprintHardness" (`/Game/SM_Project/AFB/Blueprints/FootprintTypeBase.3d Hardness` (`self.ActiveFootprintType`))))))
                        (:`B`
                          (if (< (.z _rightfootlocation) _z)
                            (for _ (range 2) :!label _label_5
                              (`/Engine/EditorBlueprintResources/StandardMacros.FlipFlop`
                                (:`A`
                                  (set `self.CurrentFootPrintLoc` (`SceneComponent.GetSocketLocation` _mesh "ball_r"))
                                  (goto _label_4))
                                (:`B`
                                  (set `self.CurrentFootPrintLoc` (`SceneComponent.GetSocketLocation` _mesh "foot_r"))
                                  (goto _label_4))))))))
                    (else
                      (goto _label_2))))
                (:`then_1`
                  ;[0.1769 0.7436 0.995 0.2] Adds Final Footprints when stopped
                  ;;[1 1 1] Checks If player is moving if not does additional imprint after short delay
                  (if (== (`KismetMathLibrary.VSize` (`CharacterMovementComponent.GetCurrentAcceleration` (`Character.CharacterMovement` (`self.CharacterReference`)))) 0.0)
                    (`/Engine/EditorBlueprintResources/StandardMacros.DoOnce` false :!label _label_6
                      (:`Completed`
                        (`KismetSystemLibrary.Delay` 0.2)
                        (`|ExecutionSequence`
                          (:`then_0`
                            (goto _label_3))
                          (:`then_1`
                            (goto _label_5)))))
                    (else
                      ;;[1 1 1] checks if player is moving faster than 30 units if so resets Do Once to enable imprint on stop
                      (if (>= (`KismetMathLibrary.VSize` (`CharacterMovementComponent.GetCurrentAcceleration` (`Character.CharacterMovement` (`self.CharacterReference`)))) 30.0)
                        (goto _label_6 :!via `Reset`)))))))))))))

(event `self.ReceiveTick`
  (params (DeltaSeconds :type "Float (single-precision)"))
  ;[0.1769 0.7436 0.995 0.2] Tick delay to increase performance
  (`KismetSystemLibrary.Delay` (`self.3dFootprintDelay`))
  ;[0.1769 0.7436 0.995 0.2] Checks if Active Footprint is Valid
  (`/Engine/EditorBlueprintResources/StandardMacros.IsValid` (`self.ActiveFootprintType`)
    (:`Is Valid`
      (`|ExecutionSequence`
        (:`then_0`
          (goto _label))
        (:`then_1`
          ;[0.1769 0.7436 0.995 0.2] Enables Elastic Footprint Tick
          (if (`/Game/SM_Project/AFB/Blueprints/FootprintTypeBase.EnableElasticFootprints` (`self.ActiveFootprintType`))
            ;[0.1769 0.7436 0.995 0.2] Current Foot Location Set On Tick used for foliage
            (`KismetMaterialLibrary.SetVectorParameterValue` "/Game/SM_Project/AFB/CollectionParams/ActiveFootLocations.ActiveFootLocations" "ElasticBigLocation" (`KismetMathLibrary.Conv_VectorToLinearColor` (`SceneComponent.K2_GetComponentLocation` (`Character.Mesh` (`self.CharacterReference`)))))
            (`KismetMaterialLibrary.SetVectorParameterValue` "/Game/SM_Project/AFB/CollectionParams/ActiveFootLocations.ActiveFootLocations" "LeftFoot" (`KismetMathLibrary.Conv_VectorToLinearColor` (`self.GetFootLocation`)))
            (`KismetMaterialLibrary.SetVectorParameterValue` "/Game/SM_Project/AFB/CollectionParams/ActiveFootLocations.ActiveFootLocations" "RightFoot" (`KismetMathLibrary.Conv_VectorToLinearColor` (`.RightfootLocation` (`self.GetFootLocation`))))
            ;[0.1769 0.7436 0.995 0.2] Sets Elastic Radius and Hardness Based on Active Footprint Setting
            (`KismetMaterialLibrary.SetScalarParameterValue` "/Game/SM_Project/AFB/CollectionParams/ActiveFootLocations.ActiveFootLocations" "ElasticFootRadius" (`/Game/SM_Project/AFB/Blueprints/FootprintTypeBase.ElasticFootRadius` (`self.ActiveFootprintType`)))
            (`KismetMaterialLibrary.SetScalarParameterValue` "/Game/SM_Project/AFB/CollectionParams/ActiveFootLocations.ActiveFootLocations" "ElasticFootHardness" (`/Game/SM_Project/AFB/Blueprints/FootprintTypeBase.ElasticFootHardness` (`self.ActiveFootprintType`)))
            (`KismetMaterialLibrary.SetScalarParameterValue` "/Game/SM_Project/AFB/CollectionParams/ActiveFootLocations.ActiveFootLocations" "ElasticBigRadius" (`/Game/SM_Project/AFB/Blueprints/FootprintTypeBase.ElasticBigRadius` (`self.ActiveFootprintType`)))
            (`KismetMaterialLibrary.SetScalarParameterValue` "/Game/SM_Project/AFB/CollectionParams/ActiveFootLocations.ActiveFootLocations" "ElasticBigHardness" (`/Game/SM_Project/AFB/Blueprints/FootprintTypeBase.ElasticBigHardness` (`self.ActiveFootprintType`)))))
        (:`then_2`
          ;[0.1769 0.7436 0.995 0.2] Enables Foliage Footrpint Tick
          (if (`/Game/SM_Project/AFB/Blueprints/FootprintTypeBase.EnableFoliagePush` (`self.ActiveFootprintType`))
            _))))))

(fn `GetFootprintTypeFromPhysicalMaterial`
  (params (PhysicalMaterial :type "PhysicalMaterial Object Reference"))
  (returns (FootprintType :type "/Game/SM_Project/AFB/Blueprints/FootprintTypeBase Object Reference"))
  (locals (PhyMatIter :type "PhysicalMaterial Object Reference") (FtTypIter :type "/Game/SM_Project/AFB/Blueprints/FootprintTypeBase Object Reference"))
  (for _array_element (`self.FootprintTypes`)
    (if (== (`/Game/SM_Project/AFB/Blueprints/FootprintTypeBase.PhysicalMaterial` _array_element) PhysicalMaterial)
      (return _array_element)))
  (return null))

(fn `OnFootFall`
  (params (Location :type "Vector Structure") (Rotation :type "Rotator Structure") (FootType :type "/Game/SM_Project/AFB/Blueprints/ENEFootType Enum"))
  (locals (NewFootprintType :type "/Game/SM_Project/AFB/Blueprints/FootprintTypeBase Object Reference"))
  (bind _outhit (`KismetSystemLibrary.LineTraceSingle` (+ Location (0.0 0.0 20.0)) (+ Location (0.0 0.0 -20.0)) "TraceTypeQuery1" true))
  ;[0.1769 0.7436 0.995 0.2] False if Falling
  (if (`GameplayStatics.BreakHitResult` _outhit)
    (bind _output_get (set `local.NewFootprintType` (`self.GetFootprintTypeFromPhysicalMaterial` (`.PhysMat` (`GameplayStatics.BreakHitResult` _outhit)))))
    (`/Engine/EditorBlueprintResources/StandardMacros.IsValid` _output_get
      (:`Is Valid`
        (if (not (== (`local.NewFootprintType`) (`self.ActiveFootprintType`)))
          (`self.OnFootprintTypeChange` (`self.ActiveFootprintType`) (`local.NewFootprintType`)))
        ;[0.1769 0.7436 0.995 0.2] Set Velocity, Max Speed , Friction, braking
        (`self.SetCharacterMovement`)
        (`/Game/SM_Project/AFB/Blueprints/FootprintTypeBase.OnFootfall` (`self.ActiveFootprintType`) (`.Location` (`GameplayStatics.BreakHitResult` _outhit)) Rotation FootType self)
        (`self.OnFootFallEvent`)))))

(fn `OnFootprintTypeChange`
  (params (OldType :type "/Game/SM_Project/AFB/Blueprints/FootprintTypeBase Object Reference") (NewType :type "/Game/SM_Project/AFB/Blueprints/FootprintTypeBase Object Reference"))
  (set `self.PreviousFootprintType` OldType)
  (set `self.ActiveFootprintType` NewType))

(fn `PlayBasicFootprintSound`
  (params (Location :type "Vector Structure") (Sound :type "SoundBase Object Reference") (SpeedVolumeMultiplier :type "Float (double-precision)"))
  ;[0.1769 0.7436 0.995 0.2] Volume Based on Speed + Random Range
  (bind _ascharacter (cast `Character` (`self.GetOwner`)))
  (bind _asblueprint_player (cast `/Game/Fix_Version/Player/Blueprint_Player` (`self.CharacterReference`))
    (:`then`
      (`/Game/Fix_Version/Player/Blueprint_Player.Ref_FootStepSound` _asblueprint_player Sound Location (+ (* SpeedVolumeMultiplier (+ (`KismetMathLibrary.RandomFloatInRange` -0.2 0.2) (/ (`KismetMathLibrary.VSize` (`Actor.GetVelocity` _ascharacter)) 500.0))) 1.0)))
    (:`CastFailed`
      (`KismetSystemLibrary.PrintString` "cast failed"))))

(fn `ResetTrackingAndMat`
  (params (Value :type "Texture Object Reference"))
  ;[0.1769 0.7436 0.995 0.2] Resets Tracking and Char Material
  (set `self.trackOpacity` 1.0)
  (set `self.NumberOfTrackSteps` 0)
  (bind _asthird_person_character_2 (cast `/Game/SM_Project/AFB/ExampleContent/Characters/ThirdPersonBP/Blueprints/ThirdPersonCharacter_2` (`GameplayStatics.GetPlayerCharacter` 0))
    (:`then`
      (bind _charactermaterial (`/Game/SM_Project/AFB/ExampleContent/Characters/ThirdPersonBP/Blueprints/ThirdPersonCharacter_2.CharacterMaterial` _asthird_person_character_2))
      (`MaterialInstanceDynamic.SetTextureParameterValue` _charactermaterial "CharcterBlendMat" Value)
      (`MaterialInstanceDynamic.SetScalarParameterValue` _charactermaterial "CharTextureLERP" (`self.trackOpacity`)))
    (:`CastFailed`
      _))
  (return))

(fn `SetCharacterMaterial`
  (params (CharacterAddTexture :type "Texture2D Object Reference"))
  ;[0.1769 0.7436 0.995 0.2] Sets the character material
  (bind _asthird_person_character_2 (cast `/Game/SM_Project/AFB/ExampleContent/Characters/ThirdPersonBP/Blueprints/ThirdPersonCharacter_2` (`GameplayStatics.GetPlayerCharacter` 0)))
  (bind _charactermaterial (`/Game/SM_Project/AFB/ExampleContent/Characters/ThirdPersonBP/Blueprints/ThirdPersonCharacter_2.CharacterMaterial` _asthird_person_character_2))
  (`MaterialInstanceDynamic.SetTextureParameterValue` _charactermaterial "CharcterBlendMat" CharacterAddTexture)
  (`MaterialInstanceDynamic.SetScalarParameterValue` _charactermaterial "CharTextureLERP" (`self.trackOpacity`))
  (set `self.ActiveFootprint` CharacterAddTexture))

(fn `SetCharacterMovement`)

(fn `SpawnDecal`
  (params (Location :type "Vector Structure") (Rotation :type "Float (double-precision)") (Size :type "Vector Structure") (Material :type "MaterialInterface Object Reference") (Lifespan :type "Float (double-precision)") (OriginalOpacity :type "Float (double-precision)"))
  ;[0.1769 0.7436 0.995 0.2] If Fade Out True spawn Actor footprint, If Fade out false spawn decal footprint
  (if (`/Game/SM_Project/AFB/Blueprints/FootprintTypeBase.Enable Decal Fade Out` (`self.ActiveFootprintType`))
    (if (not (== Material null))
      (bind _returnvalue (`|SpawnActorFromClass` "/Game/SM_Project/AFB/Blueprints/FootPrintDecal.FootPrintDecal_C" (`KismetMathLibrary.MakeTransform` Location (struct) (1.0 1.0 1.0)) "Undefined" "OverrideRootScale"))
      (set `/Game/SM_Project/AFB/Blueprints/FootPrintDecal.TimeDelay` (- Lifespan 20.0) _returnvalue)
      (set `/Game/SM_Project/AFB/Blueprints/FootPrintDecal.FootprintOriginalOpacity` OriginalOpacity _returnvalue)
      (set `/Game/SM_Project/AFB/Blueprints/FootPrintDecal.FootprintDecalMaterial` Material _returnvalue)
      (set `/Game/SM_Project/AFB/Blueprints/FootPrintDecal.FootprintSortOrder` (`/Game/SM_Project/AFB/Blueprints/FootprintTypeBase.DecalSortOrder` (`self.ActiveFootprintType`)) _returnvalue)
      (bind _decal (`/Game/SM_Project/AFB/Blueprints/FootPrintDecal.Decal` _returnvalue))
      (`SceneComponent.K2_SetWorldRotation` _decal (`KismetMathLibrary.MakeRotator` Rotation -90.0) false false)
      (`SceneComponent.SetWorldScale3D` _decal Size)
      ;[0.1769 0.7436 0.995 0.2] Sets footprint fade actor sort order
      (`DecalComponent.SetSortOrder` _decal (`/Game/SM_Project/AFB/Blueprints/FootprintTypeBase.DecalSortOrder` (`self.ActiveFootprintType`))))
    (else
      (bind _returnvalue_2 (`GameplayStatics.SpawnDecalAtLocation` Material Size Location (`KismetMathLibrary.MakeRotator` Rotation -90.0) Lifespan))
      (`/Engine/EditorBlueprintResources/StandardMacros.IsValid` _returnvalue_2
        (:`Is Valid`
          ;[0.1769 0.7436 0.995 0.2] Sets Decal Sort Order
          (`DecalComponent.SetSortOrder` _returnvalue_2 (`/Game/SM_Project/AFB/Blueprints/FootprintTypeBase.DecalSortOrder` (`self.ActiveFootprintType`)))))))
  (set `self.CurrentFootPrintLoc` Location))

(fn `SpawnParticles`
  (params (Location :type "Vector Structure") (Rotation :type "Rotator Structure") (ParticleSystem :type "ParticleSystem Object Reference"))
  (`GameplayStatics.SpawnEmitterAtLocation` ParticleSystem Location Rotation))

(fn `SpawnTracking`
  (params (Location :type "Vector Structure") (Rotation :type "Float (double-precision)") (Size :type "Vector Structure") (LifeSpan :type "Float (double-precision)") (BodyOverlayTexture :type "Texture2D Object Reference") (TrackingMat :type "MaterialInterface Object Reference") (TrackingFootprintSound :type "SoundBase Object Reference"))
  (bind _trackingsound (`self.TrackingSound`))
  (set `self.BodyOverlayTexture` BodyOverlayTexture)
  ;[0.1769 0.7436 0.995 0.2] is Tracking Enabled?
  (if (`/Game/SM_Project/AFB/Blueprints/FootprintTypeBase.EnableTracking` (`self.ActiveFootprintType`))
    ;[0.1769 0.7436 0.995 0.2] Set Tracking
    (set `self.FadeOutStepNumber` (`/Game/SM_Project/AFB/Blueprints/FootprintTypeBase.NumberOfStepsToFadeOut` (`self.ActiveFootprintType`)))
    (`self.ResetTrackingAndMat` (`self.BodyOverlayTexture`))
    (set `self.AllowTrackPrints` true)
    (set `self.ActiveTrackMaterial` (`/Game/SM_Project/AFB/Blueprints/FootprintTypeBase.FootTrackDecal` (`self.ActiveFootprintType`)))
    (if (== TrackingFootprintSound null)
      (set `self.TrackingSound` null)
      (else
        (set `self.TrackingSound` TrackingFootprintSound)))
    (else
      ;[0.1769 0.7436 0.995 0.2] checks numbers of steps
      (if (>= (`self.NumberOfTrackSteps`) (`self.FadeOutStepNumber`))
        ;[0.1769 0.7436 0.995 0.2] Reset Tracking
        (`self.ResetTrackingAndMat` (`self.BodyOverlayTexture`))
        (set `self.AllowTrackPrints` false)
        (else
          ;[0.1769 0.7436 0.995 0.2] checks if Track Prints Allowed
          (if (`self.AllowTrackPrints`)
            ;[0.1769 0.7436 0.995 0.2] Counts steps reduces opacity
            (set `self.NumberOfTrackSteps` (+ (`self.NumberOfTrackSteps`) 1))
            (set `self.trackOpacity` (- (`self.trackOpacity`) (/ 1.0 (`KismetMathLibrary.Conv_IntToDouble` (`self.FadeOutStepNumber`)))))
            ;[0.1769 0.7436 0.995 0.2] Set Character Texture Lerp
            (bind _asthird_person_character_2 (cast `/Game/SM_Project/AFB/ExampleContent/Characters/ThirdPersonBP/Blueprints/ThirdPersonCharacter_2` (`self.CharacterReference`))
              (:`then`
                (`MaterialInstanceDynamic.SetScalarParameterValue` (`/Game/SM_Project/AFB/ExampleContent/Characters/ThirdPersonBP/Blueprints/ThirdPersonCharacter_2.CharacterMaterial` _asthird_person_character_2) "CharTextureLERP" (`self.trackOpacity`)))
              (:`CastFailed`
                _))
            ;[0.1769 0.7436 0.995 0.2] play Tracking Sound
            (`/Engine/EditorBlueprintResources/StandardMacros.IsValid` _trackingsound
              (:`Is Valid`
                (`GameplayStatics.PlaySoundAtLocation` _trackingsound Location (struct) (`self.trackOpacity`)))
              (:`Is Not Valid`
                _))
            ;[0.1769 0.7436 0.995 0.2] Spawn Decal
            (`self.SpawnDecal` Location (+ Rotation 90.0) Size (`self.ActiveTrackMaterial`) LifeSpan (`self.trackOpacity`))))))))