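; ItemSpawnPoint is a placed marker that spawns one random world item, such as a healing item, hat or weapon, at its transform.
; On BeginPlay, only the authority rolls an eight-way random switch, with repeated entries weighting bandages and hats higher.
; A preceding two-way random switch has no effect because both branches lead to the same item roll.
; SpawnItem creates the chosen actor, then destroys the spawn point.
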(event `self.ReceiveBeginPlay`
  (`/Engine/EditorBlueprintResources/ActorMacros.Switch Has Authority`
    (:`Authority`
      (switch `int` (`KismetMathLibrary.RandomInteger` 2)
        (:`0`
          _)
        (:`1`
          _))
      (switch `int` (`KismetMathLibrary.RandomInteger` 8)
        (:`0`
          (`self.SpawnItem` "/Game/SM_Project/InventorySample/BluePrints/Inventory/WorldActors/Item_WorldActor_FirstAidKit.Item_WorldActor_FirstAidKit_C"))
        (:`1`
          (`self.SpawnItem` "/Game/SM_Project/InventorySample/BluePrints/Inventory/WorldActors/Item_WorldActor_Bandage.Item_WorldActor_Bandage_C"))
        (:`2`
          (`self.SpawnItem` "/Game/SM_Project/InventorySample/BluePrints/Inventory/WorldActors/Item_WorldActor_hatsix.Item_WorldActor_hatsix_C"))
        (:`3`
          (`self.SpawnItem` "/Game/Fix_Version/Weapons/Blueprint_AR413.Blueprint_AR413_C"))
        (:`4`
          (`self.SpawnItem` "/Game/Fix_Version/Weapons/Blueprint_SR413.Blueprint_SR413_C"))
        (:`5`
          (`self.SpawnItem` "/Game/SM_Project/InventorySample/BluePrints/Inventory/WorldActors/Item_WorldActor_hatsix.Item_WorldActor_hatsix_C"))
        (:`6`
          (`self.SpawnItem` "/Game/SM_Project/InventorySample/BluePrints/Inventory/WorldActors/Item_WorldActor_hatsix.Item_WorldActor_hatsix_C"))
        (:`7`
          (`self.SpawnItem` "/Game/SM_Project/InventorySample/BluePrints/Inventory/WorldActors/Item_WorldActor_Bandage.Item_WorldActor_Bandage_C"))))))

(fn `SpawnItem`
  (params (Item :type "Actor Class Reference"))
  (`|SpawnActorFromClass` Item (`self.GetTransform`) "Undefined" "OverrideRootScale")
  (`self.K2_DestroyActor`))

(fn `UserConstructionScript`)