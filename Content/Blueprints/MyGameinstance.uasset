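; Game instance that acts as the hub for menu UI and multiplayer session flow.
; Events create and show menu widgets, mostly caching them, while join and server-list widgets are rebuilt each call; favorites and chat box only reach the viewport once already created.
; LaunchGame creates an Advanced Session tagged with server and map names, then opens the map as a listen server.
; JoinServer shows the loading screen before joining; DestroySessionCaller tears sessions down.
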(event `ShowMainMenu`
  (bind _returnvalue (`GameplayStatics.GetPlayerController` 0))
  ;[1 1 1] 메인메뉴랑 마우스 커버 보여주기
  (`/Engine/EditorBlueprintResources/StandardMacros.IsValid` (`self.MainMenuWB`)
    (:`Is Valid`
      _)
    (:`Is Not Valid`
      (bind _returnvalue_2 (`|CreateWidget` "/Game/Blueprints/MainMenu.MainMenu_C" _returnvalue))
      (set `self.MainMenuWB` _returnvalue_2)))
  (`UserWidget.AddToViewport` (`self.MainMenuWB`) 0)
  (set `PlayerController.bShowMouseCursor` true _returnvalue))

(event `ShowLoadingScreen`
  ;[1 1 1] 로딩스크린 출력
  (`/Engine/EditorBlueprintResources/StandardMacros.IsValid` (`self.LoadingScreenWB`)
    (:`Is Valid`
      _)
    (:`Is Not Valid`
      (bind _returnvalue (`|CreateWidget` "/Game/Blueprints/LoadingScreen.LoadingScreen_C" (`GameplayStatics.GetPlayerController` 0)))
      (set `self.LoadingScreenWB` _returnvalue)))
  (`UserWidget.AddToViewport` (`self.LoadingScreenWB`) 3))

(event `HostMenu`
  ;[1 1 1] 방 생성 메뉴 (호스트 메뉴)
  (`/Engine/EditorBlueprintResources/StandardMacros.IsValid` (`self.HostMenuWB`)
    (:`Is Valid`
      _)
    (:`Is Not Valid`
      (bind _returnvalue (`|CreateWidget` "/Game/Blueprints/HostMenu.HostMenu_C" (`GameplayStatics.GetPlayerController` 0)))
      (set `self.HostMenuWB` _returnvalue)))
  (`UserWidget.AddToViewport` (`self.HostMenuWB`) 0))

(event `LaunchGame`
  (params (NumOfPlayer :type Integer) (`EnableLan?` :type Boolean) (ServcerName :type String))
  ;[1 1 1] 방 생성하기
  (set `self.MaxPlayers` NumOfPlayer)
  (set `self.ServerName` ServcerName)
  (`CreateSessionCallbackProxyAdvanced.CreateAdvancedSession` (`|MakeArray` (`AdvancedSessionsLibrary.MakeLiteralSessionPropertyString` "servername" (`self.ServerName`)) (`AdvancedSessionsLibrary.MakeLiteralSessionPropertyString` "MapName" (`KismetStringLibrary.Conv_NameToString` (`self.MapName`)))) (`GameplayStatics.GetPlayerController` 0) (`self.MaxPlayers`) 0 `EnableLan?`
    (:`then`
      (`GameplayStatics.OpenLevel` (`self.MapName`) true "listen"))
    (:`OnFailure`
      (`KismetSystemLibrary.PrintString` "Fail to Create Session"))))

(event `JoinMenu`
  ;[1 1 1] 방 찾기 메뉴 보여주기
  (bind _returnvalue (`|CreateWidget` "/Game/Blueprints/JoinMenu.JoinMenu_C" (`GameplayStatics.GetPlayerController` 0)))
  (set `self.JoinMenuWB` _returnvalue)
  (`UserWidget.AddToViewport` (`self.JoinMenuWB`) 0))

(event `FavoritesMenu`
  ;[1 1 1] 즐겨찾기 목록 보여주기
  (`/Engine/EditorBlueprintResources/StandardMacros.IsValid` (`self.FavoritesMenuWB`)
    (:`Is Valid`
      (`UserWidget.AddToViewport` (`self.FavoritesMenuWB`) 0))
    (:`Is Not Valid`
      (bind _returnvalue (`|CreateWidget` "/Game/Blueprints/FavoritesButton.FavoritesButton_C" (`GameplayStatics.GetPlayerController` 0)))
      (set `self.FavoritesMenuWB` _returnvalue))))

(event `DestroySessionCaller`
  (params (NewParam :type "PlayerController Object Reference"))
  ;[1 1 1] 호출 시 세션 파기
  (`DestroySessionCallbackProxy.DestroySession` NewParam))

(event `JoinServer`
  (params (SessionToJoin :type "BlueprintSessionResult Structure"))
  ;[1 1 1] 방 접속
  (`self.ShowLoadingScreen`)
  (`JoinSessionCallbackProxy.JoinSession` (`GameplayStatics.GetPlayerController` 0) SessionToJoin))

(event `ServerMenu`
  ;[1 1 1] 방 목록 보여주기 - 명령 시마다 새로 만들어 새로고침 효과 부여
  (bind _returnvalue (`|CreateWidget` "/Game/Blueprints/ServerButton.ServerButton_C" (`GameplayStatics.GetPlayerController` 0)))
  (`UserWidget.AddToViewport` _returnvalue 0))

(event `OptionMenu`
  ;[1 1 1] 옵션 창 보여주기
  (`/Engine/EditorBlueprintResources/StandardMacros.IsValid` (`self.OptionMenuWB`)
    (:`Is Valid`
      _)
    (:`Is Not Valid`
      (bind _returnvalue (`|CreateWidget` "/Game/Blueprints/OptionMenu.OptionMenu_C" (`GameplayStatics.GetPlayerController` 0)))
      (bind _returnvalue_2 (`GameUserSettings.GetGameUserSettings`))
      (bind (_x _y) (break `IntPoint` (`GameUserSettings.GetScreenResolution` _returnvalue_2)))
      (set `self.ScreenSize` (`KismetStringLibrary.Concat_StrStr` (`KismetStringLibrary.Conv_IntToString` _x) "x" (`KismetStringLibrary.Conv_IntToString` _y)))
      (set `self.OptionMenuWB` _returnvalue)))
  (`UserWidget.AddToViewport` (`self.OptionMenuWB`) 3))

(event `Chatbox`
  ;[1 1 1] 채팅창 만들기
  (`/Engine/EditorBlueprintResources/StandardMacros.IsValid` (`self.ChatBoxWB`)
    (:`Is Valid`
      (`UserWidget.AddToViewport` (`self.ChatBoxWB`) 0))
    (:`Is Not Valid`
      (bind _returnvalue (`|CreateWidget` "/Game/Blueprints/ChatBox.ChatBox_C" (`GameplayStatics.GetPlayerController` 0)))
      (set `self.ChatBoxWB` _returnvalue))))