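; Actor component that drives a stealth-field effect on stealth and distortion meshes, with timed or instant toggling.
; Activate, deactivate and break events set Efficiency and Distortion targets, which Tick lerps toward before updating state flags.
; Setters push these values and glow settings through dynamic material instances, and distortion meshes hide after unstealthing.
; Damage raises target distortion, breaking the field with a glow spike and faster fade past 1.0.
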(event `self.ReceiveTick`
  (params (DeltaSeconds :type "Float (single-precision)"))
  (bind _returnvalue (+ (`self.DistortionLerp`) (/ DeltaSeconds (`self.Duration`))))
  (bind _returnvalue_2 (+ (`self.EfficiencyLerp`) (/ DeltaSeconds (`self.Duration`))))
  ;[1 1 1] Tick
  (`|ExecutionSequence`
    (:`then_0`
      ;;[1 1 1] If the current efficiency doesn't match the target efficiency, we have some changes to make.
      (if (!= (`self.CurrentEfficiency`) (`self.TargetEfficiency`))
        ;;[1 1 1] Move the efficiency closer to target efficiency, over a period of Duration seconds
        (if (> _returnvalue_2 1.0)
          (set `self.EfficiencyLerp` 0.0)
          (set `self.CurrentEfficiency` (`self.TargetEfficiency`))
          (else
            (set `self.EfficiencyLerp` _returnvalue_2)
            (set `self.CurrentEfficiency` (`KismetMathLibrary.Lerp` (`self.StartingEfficiency`) (`self.TargetEfficiency`) (`self.EfficiencyLerp`)))))
        (`self.SetEfficiencies` (`self.CurrentEfficiency`))))
    (:`then_1`
      ;;[1 1 1] If the current distortion doesn't match the target distortion, we have some changes to make.
      (if (!= (`self.CurrentDistortion`) (`self.TargetDistortion`))
        ;;[1 1 1] Move the distortion closer to target distortion, over a period of Duration seconds
        (if (> _returnvalue 1.0)
          (set `self.DistortionLerp` 0.0)
          (set `self.CurrentDistortion` (`self.TargetDistortion`))
          (else
            (set `self.DistortionLerp` _returnvalue)
            (set `self.CurrentDistortion` (`KismetMathLibrary.Lerp` (`self.StartingDistortion`) (`self.TargetDistortion`) (`self.DistortionLerp`)))))
        (`self.SetDistortions` (`self.CurrentDistortion`))))
    (:`then_2`
      (if (and (== (`self.CurrentEfficiency`) (`self.TargetEfficiency`)) (== (`self.CurrentDistortion`) (`self.TargetDistortion`)))
        (if (`self.bIsStealthing`)
          (set `self.bIsStealthing` false)
          (set `self.bIsStealthed` true)
          (elif (`self.bIsUnstealthing`)
            (set `self.bIsUnstealthing` false)
            ;;[1 1 1] Set distortion mesh to invisible as an extra precaution
            (for _array_element (`self.DistortionMeshes`)
              (bind _asprimitive_component (cast `PrimitiveComponent` _array_element)
                (:`then`
                  (`self.SetVisibility` _asprimitive_component false false))
                (:`CastFailed`
                  ;;[1 1 1] Error Logging
                  (`KismetSystemLibrary.PrintString` (`KismetStringLibrary.Concat_StrStr` "ERROR: Cast to PrimitiveComponent failed for " (`KismetSystemLibrary.GetObjectName` _array_element) " in " (`KismetSystemLibrary.GetObjectName` self) " Event Tick.") true true (struct :`R` 1.0 :`A` 1.0)))))))))))

(event `self.ReceiveBeginPlay`
  (`self.SetComponentTickEnabled` true))

(event `SetEfficiencies`
  (params (Efficiency :type "Float (double-precision)"))
  ;[1 1 1] Set stealth mesh efficiencies
  (for _array_element (`self.StealthMeshes`)
    (bind _asprimitive_component (cast `PrimitiveComponent` _array_element)
      (:`then`
        (for _index (range (`PrimitiveComponent.GetNumMaterials` _asprimitive_component))
          (bind _returnvalue (`PrimitiveComponent.CreateDynamicMaterialInstance` _asprimitive_component _index (`PrimitiveComponent.GetMaterial` _asprimitive_component _index)))
          (`MaterialInstanceDynamic.SetScalarParameterValue` _returnvalue "Efficiency" Efficiency)))
      (:`CastFailed`
        ;[1 1 1] Error Logging
        (`KismetSystemLibrary.PrintString` (`KismetStringLibrary.Concat_StrStr` "ERROR: Cast to PrimitiveComponent failed for " (`KismetSystemLibrary.GetObjectName` _array_element) " in " (`KismetSystemLibrary.GetObjectName` self) " SetEfficiencies.") true true (struct :`R` 1.0 :`A` 1.0))))))

(event `BreakStealthField`
  ;[1 1 1] Break the stealth field
  (`|ExecutionSequence`
    (:`then_0`
      (`self.SetGlowIntensities` (* (`self.GlowIntensity`) 100.0))
      (set `self.Duration` (/ (`self.DefaultDuration`) 10.0))
      (set `self.bIsUnstealthing` true)
      (set `self.bIsStealthed` false))
    (:`then_1`
      (set `self.StartingEfficiency` (`self.CurrentEfficiency`))
      (set `self.TargetEfficiency` 0.0))
    (:`then_2`
      (set `self.StartingDistortion` (`self.CurrentDistortion`))
      (set `self.TargetDistortion` 0.0))))

(event `ActivateStealthField`
  ;[1 1 1] Activate stealth field
  (`|ExecutionSequence`
    (:`then_0`
      (set `self.bIsStealthing` true)
      (set `self.Duration` (`self.DefaultDuration`)))
    (:`then_1`
      (set `self.StartingEfficiency` 0.0)
      (set `self.CurrentEfficiency` 0.0)
      (set `self.TargetEfficiency` 1.0))
    (:`then_2`
      (set `self.CurrentDistortion` 0.0)
      (set `self.TargetDistortion` (`self.DefaultDistortion`))
      (set `self.StartingDistortion` 0.0))
    (:`then_3`
      (`self.SetGlowIntensities` (`self.GlowIntensity`))
      (`self.SetGlowColor` (`self.GlowColor`))
      (`self.SetFringeSizes` (`self.GlowFringeSize`)))
    (:`then_4`
      (`self.SetDistortionVisibleForAll`))))

(event `DeactivateStealthField`
  ;[1 1 1] Deactivate stealth field
  (`|ExecutionSequence`
    (:`then_0`
      (set `self.bIsUnstealthing` true)
      (set `self.Duration` (`self.DefaultDuration`))
      (set `self.bIsStealthed` false))
    (:`then_1`
      (set `self.StartingEfficiency` (`self.CurrentEfficiency`))
      (set `self.StartingDistortion` (`self.CurrentDistortion`)))
    (:`then_2`
      (set `self.TargetEfficiency` 0.0)
      (set `self.TargetDistortion` 0.0))))

(event `SetDistortions`
  (params (Distortion :type "Float (double-precision)"))
  ;[1 1 1] Set distortion mesh distortions
  (for _array_element (`self.DistortionMeshes`)
    (bind _asprimitive_component (cast `PrimitiveComponent` _array_element)
      (:`then`
        (for _index (range (`PrimitiveComponent.GetNumMaterials` _asprimitive_component))
          (bind _returnvalue (`PrimitiveComponent.CreateDynamicMaterialInstance` _asprimitive_component _index (`PrimitiveComponent.GetMaterial` _asprimitive_component _index)))
          (`MaterialInstanceDynamic.SetScalarParameterValue` _returnvalue "Distortion" Distortion)))
      (:`CastFailed`
        ;[1 1 1] Error Logging
        (`KismetSystemLibrary.PrintString` (`KismetStringLibrary.Concat_StrStr` "ERROR: Cast to PrimitiveComponent failed for " (`KismetSystemLibrary.GetObjectName` _array_element) " in " (`KismetSystemLibrary.GetObjectName` self) " SetDistortions.") true true (struct :`R` 1.0 :`A` 1.0))))))

(event `SetDistortionVisibleForAll`
  ;[1 1 1] Set distortion mesh to visible to allow distortion effect
  (for _array_element (`self.DistortionMeshes`)
    (bind _asprimitive_component (cast `PrimitiveComponent` _array_element)
      (:`then`
        (`self.SetVisibility` _asprimitive_component true false))
      (:`CastFailed`
        ;[1 1 1] Error Logging
        (`KismetSystemLibrary.PrintString` (`KismetStringLibrary.Concat_StrStr` "ERROR: Cast to PrimitiveComponent failed for " (`KismetSystemLibrary.GetObjectName` _array_element) " in " (`KismetSystemLibrary.GetObjectName` self) " Event Tick.") true true (struct :`R` 1.0 :`A` 1.0))))))

(event `ToggleStealth`
  ;[1 1 1] Toggle the stealth field
  (if (or (`self.bIsStealthing`) (`self.bIsUnstealthing`))
    _
    (elif (`self.bIsStealthed`)
      (`self.DeactivateStealthField`)
      (else
        (`self.ActivateStealthField`)))))

(event `ToggleStealth_Instant`
  ;[1 1 1] Toggle the stealth field: Instant
  (if (or (`self.bIsStealthing`) (`self.bIsUnstealthing`))
    _
    (elif (`self.bIsStealthed`)
      (`self.DeactivateStealthField_Instant`)
      (else
        (`self.ActivateStealthField_Instant`)))))

(event `DeactivateStealthField_Instant`
  ;[1 1 1] Deactivate stealth field: instant
  (`|ExecutionSequence`
    (:`then_0`
      (set `self.bIsUnstealthing` true)
      (set `self.Duration` 0.0001)
      (set `self.bIsStealthed` false))
    (:`then_1`
      (set `self.StartingEfficiency` (`self.CurrentEfficiency`))
      (set `self.StartingDistortion` (`self.CurrentDistortion`)))
    (:`then_2`
      (set `self.TargetEfficiency` 0.0)
      (set `self.TargetDistortion` 0.0))))

(event `ActivateStealthField_Instant`
  ;[1 1 1] Activate stealth field: Instant
  (`|ExecutionSequence`
    (:`then_0`
      (set `self.bIsStealthing` true)
      (set `self.Duration` 0.0001))
    (:`then_1`
      (set `self.StartingEfficiency` 0.0)
      (set `self.CurrentEfficiency` 0.0)
      (set `self.TargetEfficiency` 1.0))
    (:`then_2`
      (set `self.CurrentDistortion` 0.0)
      (set `self.TargetDistortion` (`self.DefaultDistortion`))
      (set `self.StartingDistortion` 0.0))
    (:`then_3`
      (`self.SetGlowIntensities` (`self.GlowIntensity`))
      (`self.SetGlowColor` (`self.GlowColor`))
      (`self.SetFringeSizes` (`self.GlowFringeSize`)))
    (:`then_4`
      (`self.SetDistortionVisibleForAll`))))

(event `DamageStealthField`
  (params (Damage :type "Float (double-precision)"))
  (bind _returnvalue (+ Damage (`self.TargetDistortion`)))
  ;[1 1 1] Add value of Damage to the efficiency of the stealth field. If efficiency value is greater than 1.0, the stealth field breaks.
  (if (`self.bIsUnstealthing`)
    (`self.BreakStealthField` :!label _label)
    (elif (> _returnvalue 1.0)
      (goto _label)
      (else
        (set `self.TargetDistortion` _returnvalue)
        (set `self.StartingDistortion` (`self.CurrentDistortion`))
        (if (`self.bIsStealthing`)
          (set `self.Duration` (`self.DefaultDuration`))
          (else
            (set `self.Duration` (/ (`self.DefaultDuration`) 10.0))))))))

(event `SetFringeSizes`
  (params (FringeSize :type "Float (double-precision)"))
  ;[1 1 1] Set stealth material fringe sizes
  (for _array_element (`self.StealthMeshes`)
    (bind _asprimitive_component (cast `PrimitiveComponent` _array_element)
      (:`then`
        (for _index (range (`PrimitiveComponent.GetNumMaterials` _asprimitive_component))
          (bind _returnvalue (`PrimitiveComponent.CreateDynamicMaterialInstance` _asprimitive_component _index (`PrimitiveComponent.GetMaterial` _asprimitive_component _index)))
          (`MaterialInstanceDynamic.SetScalarParameterValue` _returnvalue "FringeSize" FringeSize)))
      (:`CastFailed`
        ;[1 1 1] Error Logging
        (`KismetSystemLibrary.PrintString` (`KismetStringLibrary.Concat_StrStr` "ERROR: Cast to PrimitiveComponent failed for " (`KismetSystemLibrary.GetObjectName` _array_element) " in " (`KismetSystemLibrary.GetObjectName` self) " SetFringeSizes.") true true (struct :`R` 1.0 :`A` 1.0))))))

(event `SetGlowIntensities`
  (params (GlowIntensity :type "Float (double-precision)"))
  ;[1 1 1] Set stealth material glow intensities
  (for _array_element (`self.StealthMeshes`)
    (bind _asprimitive_component (cast `PrimitiveComponent` _array_element)
      (:`then`
        (for _index (range (`PrimitiveComponent.GetNumMaterials` _asprimitive_component))
          (bind _returnvalue (`PrimitiveComponent.CreateDynamicMaterialInstance` _asprimitive_component _index (`PrimitiveComponent.GetMaterial` _asprimitive_component _index)))
          (`MaterialInstanceDynamic.SetScalarParameterValue` _returnvalue "GlowIntensity" GlowIntensity)))
      (:`CastFailed`
        ;[1 1 1] Error Logging
        (`KismetSystemLibrary.PrintString` (`KismetStringLibrary.Concat_StrStr` "ERROR: Cast to PrimitiveComponent failed for " (`KismetSystemLibrary.GetObjectName` _array_element) " in " (`KismetSystemLibrary.GetObjectName` self) " SetGlowIntensities.") true true (struct :`R` 1.0 :`A` 1.0))))))

(event `SetGlowColor`
  (params (GlowColor :type "Vector Structure"))
  (`|ExecutionSequence`
    (:`then_0`
      ;[1 1 1] Set stealth materal glow color
      (for _array_element (`self.StealthMeshes`)
        (bind _asprimitive_component (cast `PrimitiveComponent` _array_element)
          (:`then`
            (for _index (range (`PrimitiveComponent.GetNumMaterials` _asprimitive_component))
              (bind _returnvalue (`PrimitiveComponent.CreateDynamicMaterialInstance` _asprimitive_component _index (`PrimitiveComponent.GetMaterial` _asprimitive_component _index)))
              (`MaterialInstanceDynamic.SetVectorParameterValue` _returnvalue "GlowColor" (`KismetMathLibrary.Conv_VectorToLinearColor` GlowColor))))
          (:`CastFailed`
            ;[1 1 1] Error Logging
            (`KismetSystemLibrary.PrintString` (`KismetStringLibrary.Concat_StrStr` "ERROR: Cast to PrimitiveComponent failed for " (`KismetSystemLibrary.GetObjectName` _array_element) " in " (`KismetSystemLibrary.GetObjectName` self) " SetGlowColor.") true true (struct :`R` 1.0 :`A` 1.0))))))
    (:`then_1`
      ;[1 1 1] Set distortion glow color
      (for _array_element_2 (`self.DistortionMeshes`)
        (bind _asprimitive_component_2 (cast `PrimitiveComponent` _array_element_2)
          (:`then`
            (for _index_2 (range (`PrimitiveComponent.GetNumMaterials` _asprimitive_component_2))
              (bind _returnvalue_2 (`PrimitiveComponent.CreateDynamicMaterialInstance` _asprimitive_component_2 _index_2 (`PrimitiveComponent.GetMaterial` _asprimitive_component_2 _index_2)))
              (`MaterialInstanceDynamic.SetVectorParameterValue` _returnvalue_2 "GlowColor" (`KismetMathLibrary.Conv_VectorToLinearColor` GlowColor))))
          (:`CastFailed`
            ;[1 1 1] Error Logging
            (`KismetSystemLibrary.PrintString` (`KismetStringLibrary.Concat_StrStr` "ERROR: Cast to PrimitiveComponent failed for " (`KismetSystemLibrary.GetObjectName` _array_element_2) " in " (`KismetSystemLibrary.GetObjectName` self) " SetGlowColor.") true true (struct :`R` 1.0 :`A` 1.0))))))))